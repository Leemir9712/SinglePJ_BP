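; BP_Camera is a free-moving camera that shows the mouse cursor for the first player controller on BeginPlay.
; Three input axes move its Camera component forward, sideways and vertically through relative location offsets.
; Each offset is a fixed step scaled only by axis value, without delta time or sweep, so speed depends on frame rate and collisions are ignored.
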(event EventBeginPlay
  (Variables|/Script/Engine.PlayerController|SetbShowMouseCursor (Game|GetPlayerController 0) true))

(event Input|AxisEvents|InputAxisMoveForward
  (params (AxisValue :type Float%20%28single-precision%29))
  (Transformation|AddRelativeLocation (Variables|Default|GetCamera) (* "30.000000,0.000000, 0" AxisValue) false false))

(event Input|AxisEvents|InputAxisMoveRight
  (params (AxisValue :type Float%20%28single-precision%29))
  (Transformation|AddRelativeLocation (Variables|Default|GetCamera) (* "0.000000,30.000000, 0" AxisValue) false false))

(event Input|AxisEvents|InputAxisCameraUpDown
  (params (AxisValue :type Float%20%28single-precision%29))
  (Transformation|AddRelativeLocation (Variables|Default|GetCamera) (* "0.000000,0.000000,30.000000" AxisValue) false false))

(fn ConstructionScript)